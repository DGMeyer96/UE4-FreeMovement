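; Free-movement player character that can grab, hang from and climb ledges, with camera shakes for running and landing.
; While falling, Tick sphere-traces for a wall and ledge top, then switches to Flying and snaps the capsule to the wall.
; Space climbs or jumps and Crouch lets go, with grab and climb states exchanged with the AnimBP through interface messages.
; An older montage-and-teleport climb remains, unconnected.
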(event `Key|SpaceBar`
  (params (Key :type "Key Structure"))
  ;[0 1 0] Jump Handling
  (:`Pressed`
    (if (`self.bIsHanging`)
      (`self.ClimbLedge`)
      (else
        (`self.Jump`)))))

(event `self.ReceiveTick`
  (params (DeltaSeconds :type "Float (single-precision)"))
  (bind _capsulehalfheight (`CapsuleComponent.CapsuleHalfHeight` (`self.CapsuleComponent`)))
  ;[1 0 0] Tick
  (`|ExecutionSequence`
    (:`then_0`
      ;[1 1 1] Running Camera Shake
      (if (or (!= (`self.MoveForwardInput`) 0.0) (!= (`self.MoveRightInput`) 0.0))
        (`CameraShakeSourceComponent.StartCameraShake` (`self.CameraShakeSource`) "/Game/FreeMovement/Camera/Running_CameraShake.Running_CameraShake_C" 1.0 "CameraLocal" (struct))))
    (:`then_1`
      ;[0 0 1] Check for Wall and Ledge
      (`self.CanCheckForWall`
        (:`Out`
          (bind (_out_hitwall _out_wallimpactpoint _out_wallimpactnormal) (`self.WallCheck`))
          (if _out_hitwall
            (set `self.Wall Impact Point` _out_wallimpactpoint)
            (set `self.Wall Impact Normal` _out_wallimpactnormal)
            (bind (_out_canclimb _out_ledgelocation _out_ledgeimpactpoint) (`self.LedgeCheck`))
            (if _out_canclimb
              (set `self.Ledge Height` _out_ledgelocation)
              (set `self.LedgeLocation` _out_ledgeimpactpoint)
              ;[0 0 1] Within range of ledge, but not already grabbing
              (if (and (`self.HipDistanceToLedge` (* _capsulehalfheight -1.0) _capsulehalfheight) (not (`self.IsClimbingLedge`)))
                ;[0 0 1] Grab The Ledge
                (message `/Game/FreeMovement/CharacterMoveInterface.CanGrabLedge_BI` (`SkeletalMeshComponent.GetAnimInstance` (`self.Mesh`)) true)
                (`CharacterMovementComponent.SetMovementMode` (`self.CharacterMovement`) "MOVE_Flying" 0)
                (set `self.bIsHanging` true)
                (`KismetSystemLibrary.MoveComponentTo` (`self.CapsuleComponent`) (`self.WallGoToLocation` 75.0) (`self.AlignToWall`) false false 0.1)
                (`MovementComponent.StopMovementImmediately` (`self.CharacterMovement`))))))))))

(event `InputAction|Jump`
  (params (Key :type "Key Structure"))
  ;[0 1 0] Jump Handling
)

(event `self.ReceiveBeginPlay`
  ;[1 0 0] Begin Play
)

(event `InputAction|Crouch`
  (params (Key :type "Key Structure"))
  ;[0 1 0.013] Crouch Handling
  (:`Pressed`
    (if (`self.bIsHanging`)
      (`self.LetGoOfLedge`))))

(event `ClimbLedge`
  ;[0 0 1] Ledge Climb Start
  (if (not (`self.IsClimbingLedge`))
    (`CharacterMovementComponent.SetMovementMode` (`self.CharacterMovement`) "MOVE_Flying" 0)
    (message `/Game/FreeMovement/CharacterMoveInterface.ClimbingLedge_BI` (`SkeletalMeshComponent.GetAnimInstance` (`self.Mesh`)) true)
    (set `self.IsClimbingLedge` true)
    (set `self.bIsHanging` false)))

(event `self.OnLanded`
  (params (Hit :type "HitResult Structure (by ref)"))
  (bind (_returnvalue_x _returnvalue_y _returnvalue_z) (`KismetMathLibrary.BreakVector` (`self.GetVelocity`)))
  (bind _camerashakesource (`self.CameraShakeSource`))
  ;[0 1 0] On Landed
  (if (<= _returnvalue_z (`self.HardLandingSpeed`))
    (`CameraShakeSourceComponent.StartCameraShake` :`self` _camerashakesource :`InCameraShake` "/Game/FreeMovement/Camera/HardLanding_CameraShake.HardLanding_CameraShake_C")
    (else
      (`CameraShakeSourceComponent.StartCameraShake` :`self` _camerashakesource :`InCameraShake` "/Game/FreeMovement/Camera/Landing_CameraShake.Landing_CameraShake_C" :`Scale` 0.5))))

(event `/Game/FreeMovement/CharacterMoveInterface.ClimbingLedge_BI`
  (params (IsClimbing :type Boolean))
  ;[0 0 1] Ledge Climb End
  (set `self.IsClimbingLedge` IsClimbing)
  (`CharacterMovementComponent.SetMovementMode` (`self.CharacterMovement`) "MOVE_Walking" 0))

(event `LetGoOfLedge`
  ;[0 0 1] Let Go Of Ledge
  (`CharacterMovementComponent.SetMovementMode` (`self.CharacterMovement`) "MOVE_Walking" 0)
  (message `/Game/FreeMovement/CharacterMoveInterface.CanGrabLedge_BI` (`SkeletalMeshComponent.GetAnimInstance` (`self.Mesh`)) false)
  (set `self.bIsHanging` false))

(fn `CheckForLedgeGrab`
  (returns (CanHang :type Boolean) (HangLocation :type "Vector Structure") (HitNormal :type "Vector Structure"))
  (locals (TraceLength :type "Float (double-precision)" :default 120.0) (UpTraceDistance :type "Float (double-precision)" :default 10.0) (NumChecks :type Integer :default 10))
  (for _index (range 1 (+ (`local.NumChecks`) 1))
    (bind _returnvalue (+ (+ (`self.K2_GetActorLocation`) (0.0 0.0 90.0)) (`KismetMathLibrary.MakeVector` 0.0 0.0 (* _index (`local.UpTraceDistance`)))))
    (bind (_outhit _returnvalue_2) (`KismetSystemLibrary.SphereTraceSingle` :`Start` _returnvalue :`End` (+ _returnvalue (* (`KismetMathLibrary.GetForwardVector` (`self.K2_GetActorRotation`)) (`local.TraceLength`))) :`Radius` 10.0 :`TraceChannel` "TraceTypeQuery1" :`DrawDebugType` "ForDuration" :`DrawTime` 1.0))
    (if _returnvalue_2
      (bind _returnvalue_3 (+ (`.ImpactPoint` (`GameplayStatics.BreakHitResult` _outhit)) (0.0 0.0 20.0)))
      (bind (_outhit_2 _returnvalue_4) (`KismetSystemLibrary.SphereTraceSingle` :`Start` _returnvalue_3 :`End` (+ _returnvalue_3 (0.0 0.0 20.0)) :`Radius` 10.0 :`TraceChannel` "TraceTypeQuery1" :`DrawDebugType` "ForDuration" :`DrawTime` 1.0))
      (if (not _returnvalue_4)
        (`|ExecutionSequence`
          (:`then_0`
            (break))
          (:`then_1`
            (return true (`.ImpactPoint` (`GameplayStatics.BreakHitResult` _outhit_2)) (`.ImpactNormal` (`GameplayStatics.BreakHitResult` _outhit))))))))
  (return false (0.0 0.0 0.0) (0.0 0.0 0.0)))

(fn `LedgeCheck`
  (returns (Out_CanClimb :type Boolean) (Out_LedgeLocation :type "Vector Structure") (Out_LedgeImpactPoint :type "Vector Structure"))
  (bind _capsuleradius (`CapsuleComponent.CapsuleRadius` (`self.CapsuleComponent`)))
  (bind _returnvalue (+ (`self.K2_GetActorLocation`) (* (`self.GetActorForwardVector`) _capsuleradius)))
  (bind (_outhit _returnvalue_2) (`KismetSystemLibrary.SphereTraceSingle` :`Start` (+ _returnvalue (`KismetMathLibrary.MakeVector` 0.0 0.0 (`CharacterMovementComponent.GetMaxJumpHeight` (`self.CharacterMovement`)))) :`End` _returnvalue :`Radius` _capsuleradius :`TraceChannel` "TraceTypeQuery1" :`bTraceComplex` true :`DrawDebugType` "ForOneFrame"))
  (return _returnvalue_2 (`.Location` (`GameplayStatics.BreakHitResult` _outhit)) (`.ImpactPoint` (`GameplayStatics.BreakHitResult` _outhit))))

(fn `LedgeDistanceCheck`
  (returns (`GrabLedge?` :type Boolean))
  (return (<= (`KismetMathLibrary.VSize` (- (`self.K2_GetActorLocation`) (`self.LocationToMoveTo`))) 100.0)))

(fn `MoveToLedge`
  (`self.K2_SetActorLocation` (- (`self.LocationToMoveTo`) (* (`self.GetActorForwardVector`) (`CapsuleComponent.CapsuleRadius` (`self.CapsuleComponent`))))))

(fn `MoveToLedgeTop`
  (bind _capsulecomponent (`self.CapsuleComponent`))
  (`self.K2_SetActorLocation` (+ (+ (`self.LocationToMoveTo`) (`KismetMathLibrary.MakeVector` 0.0 0.0 (`CapsuleComponent.CapsuleHalfHeight` _capsulecomponent))) (* (`self.GetActorForwardVector`) (* (`CapsuleComponent.CapsuleRadius` _capsulecomponent) 2.0)))))

(fn `MoveToLocation`
  (bind _returnvalue (+ (.z (`self.LocationToMoveTo`)) (`CapsuleComponent.CapsuleHalfHeight` (`self.CapsuleComponent`))))
  (bind _returnvalue_2 (`KismetMathLibrary.FInterpTo` (.z (`self.K2_GetActorLocation`)) _returnvalue (`GameplayStatics.GetWorldDeltaSeconds`) 1.0))
  (if (< _returnvalue_2 _returnvalue)
    (`self.K2_SetActorLocation` (`KismetMathLibrary.MakeVector` (.x (`self.K2_GetActorLocation`)) (.y (`self.K2_GetActorLocation`)) _returnvalue_2))
    (`KismetSystemLibrary.PrintString` "Climb Up")
    (else
      (`self.K2_SetActorLocation` (+ (`self.K2_GetActorLocation`) (* (`self.GetActorForwardVector`) (`CapsuleComponent.CapsuleRadius` (`self.CapsuleComponent`)))))
      (set `self.bRunTest` false)
      (`KismetSystemLibrary.PrintString` "Move Forward"))))

(fn `UserConstructionScript`)

(fn `WallCheck`
  (returns (Out_HitWall :type Boolean) (Out_WallImpactPoint :type "Vector Structure") (Out_WallImpactNormal :type "Vector Structure"))
  (bind _returnvalue (`self.K2_GetActorLocation`))
  (bind _capsuleradius (`CapsuleComponent.CapsuleRadius` (`self.CapsuleComponent`)))
  (bind (_outhit _returnvalue_2) (`KismetSystemLibrary.SphereTraceSingle` :`Start` _returnvalue :`End` (+ _returnvalue (* (`self.GetActorForwardVector`) _capsuleradius)) :`Radius` (* _capsuleradius 1.5) :`TraceChannel` "TraceTypeQuery1" :`bTraceComplex` true :`DrawDebugType` "ForOneFrame"))
  (return _returnvalue_2 (`.ImpactPoint` (`GameplayStatics.BreakHitResult` _outhit)) (`.ImpactNormal` (`GameplayStatics.BreakHitResult` _outhit))))